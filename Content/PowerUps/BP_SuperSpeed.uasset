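; BP_SuperSpeed is a power-up that temporarily doubles the walk speed of the BP_PlayerPawn that activates it.
; On activation it stores the pawn and passes twice its current MaxWalkSpeed to both ChangeWalkSpeed and ClientChangeWalkSpeed.
; On expiry it makes the same two calls with a hardcoded default speed rather than the original value.
; Both events print an on-screen message, and the tick event is empty.
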(event EventOnActivated
  (params (Actor :type Actor%20Object%20Reference))
  (bind _asbp_player_pawn (Utilities|Casting|CastToBP_PlayerPawn Actor))
  (bind _output_get (Variables|Default|SetPlayer_Ref _asbp_player_pawn))
  (Default|ChangeWalkSpeed _output_get (* (Variables|/Script/Engine.CharacterMovementComponent|GetMaxWalkSpeed (Actor|GetComponentbyClass _asbp_player_pawn "/Script/Engine.CharacterMovementComponent")) 2.0))
  (Default|ClientChangeWalkSpeed _output_get (* (Variables|/Script/Engine.CharacterMovementComponent|GetMaxWalkSpeed (Actor|GetComponentbyClass _asbp_player_pawn "/Script/Engine.CharacterMovementComponent")) 2.0))
  (Development|PrintString "YOU GET SUPERSPEED !" true false "(R=0.043367,G=1.000000,B=0.127033,A=1.000000)"))

(event EventOnExpired
  (bind _player_ref (Variables|Default|GetPlayer_Ref))
  (Default|ChangeWalkSpeed _player_ref 6e+02)
  (Default|ClientChangeWalkSpeed _player_ref 6e+02)
  (Development|PrintString "YOU LOOSE SUPERSPEED !" true false "(R=0.043367,G=1.000000,B=0.127033,A=1.000000)"))

(event EventOnPowerUpTicked)

(fn ConstructionScript)