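; Health regeneration power-up that gradually restores health to the CSCharacter that activates it.
; On activation it stores the character reference and prints an on-screen pickup message.
; Each power-up tick adds a fixed amount directly to the character's SCHealthComponent current health, clamped between zero and max health.
; Expiry has no logic; tick timing is not set in these graphs.
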(event EventOnActivated
  (params (Actor :type Actor%20Object%20Reference))
  (bind _ascscharacter (Utilities|Casting|CastToCSCharacter Actor))
  (Variables|Default|SetPlayerRef _ascscharacter)
  (Development|PrintString (Utilities|String|Append (Utilities|GetDisplayName Actor) "  GOT HEALTH REGEN !") true false "(R=0.057292,G=1.000000,B=0.371430,A=1.000000)"))

(event EventOnPowerUpTicked
  (bind _playerref (Variables|Default|GetPlayerRef))
  (bind _returnvalue (Actor|GetComponentbyClass _playerref "/Script/CoopShooter.SCHealthComponent"))
  (Variables|/Script/CoopShooter.SCHealthComponent|SetCurrentHealth _returnvalue (Math|Float|Clamp(Float) (+ (Variables|/Script/CoopShooter.SCHealthComponent|GetCurrentHealth _returnvalue) 1e+01) 0.0 (Variables|/Script/CoopShooter.SCHealthComponent|GetMaxHealth _returnvalue))))

(event EventOnExpired)

(fn ConstructionScript)