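; Player controller that creates and drives the local player's HUD.
; On BeginPlay it caches the game state, adds a W_Hud widget to the viewport and binds to the game state's wave state change event.
; Wave changes push the current wave state enum name to the HUD, and a SetScore event forwards score values to it as text.
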(event Custom|WaveStateChange_Event_0
  (Default|SetTextWaveState (Variables|Default|GetHudWidgetRef) (Utilities|Text|ToText(String) (Utilities|String|EnumtoString (Variables|/Script/CoopShooter.CSGameStateBase|GetWaveState (Variables|Default|GetGameStateRef))))))

(event Custom|SetScore
  (params (Score :type Float%20%28single-precision%29))
  (Default|SetTextScore (Variables|Default|GetHudWidgetRef) (Utilities|Text|ToText(Float) Score "HalfToEven")))

(event EventBeginPlay
  (if (Pawn|IsLocalController)
    (bind _asbp_game_state (Utilities|Casting|CastToBP_GameState (Game|GetGameState)))
    (Variables|Default|SetGameStateRef _asbp_game_state)
    (bind _returnvalue (UserInterface|CreateWidget "/Game/UI/W_Hud.W_Hud_C" self))
    (bind _output_get (Variables|Default|SetHudWidgetRef _returnvalue))
    (UserInterface|Viewport|AddtoViewport _output_get 0)
    (EventDispatchers|AssignWaveStateChange (Variables|Default|GetGameStateRef) (delegate Custom|WaveStateChange_Event_0))))

(fn ConstructionScript)